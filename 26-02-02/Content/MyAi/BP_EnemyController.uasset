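; AI controller for the boss enemy that runs the BT_Boss behavior tree and reports death to its Blackboard.
; On possess it starts the tree, casts the pawn to BP_Boss and binds its death dispatcher to set IsDeadKey.
; A separate AnyDamage handler casts the controlled pawn to BP_MyCharacter instead, subtracts damage from CurrentHealth and sets the same key at zero or below.
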(event Custom|커스텀이벤트
  (AI|Components|Blackboard|SetValueasBool (Variables|Default|GetBlackboard) (Variables|Default|GetIsDeadKey) true))

(event EventTick
  (params (DeltaSeconds :type Float%20%28single-precision%29)))

(event EventPossess
  (params (PossessedPawn :type Pawn%20Object%20Reference))
  (AI|RunBehaviorTree "/Game/MyAi/BT_Boss.BT_Boss")
  (bind _asbp_boss (Utilities|Casting|CastToBP_Boss PossessedPawn))
  (EventDispatchers|BindEventtoOnDeadEventDispatcher _asbp_boss (delegate Custom|커스텀이벤트)))

(event Game|Damage|EventAnyDamage
  (params (Damage :type Float%20%28single-precision%29) (DamageType :type Damage%20Type%20Object%20Reference) (InstigatedBy :type Controller%20Object%20Reference) (DamageCauser :type Actor%20Object%20Reference))
  (bind _asbp_my_character (Utilities|Casting|CastToBP_MyCharacter (Pawn|GetControlledPawn)))
  (bind _output_get (Variables|/Script/Project.MyCharacter|SetCurrentHealth _asbp_my_character (- (Variables|/Script/Project.MyCharacter|GetCurrentHealth _asbp_my_character) Damage)))
  (if (<= _output_get 0.0)
    (bind _returnvalue (AI|GetAIController 0))
    (bind _returnvalue_2 (AI|GetBlackboard _returnvalue))
    (AI|Components|Blackboard|SetValueasBool _returnvalue_2 (Variables|Default|GetIsDeadKey) true)))

(fn ConstructionScript)